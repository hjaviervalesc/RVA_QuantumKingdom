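; BP_Target is a shootable target actor that counts as an enemy kill in level 2 when a projectile hits it.
; If marked mobile, it oscillates around its spawn location each tick along a normalized direction, using a sine of accumulated time scaled by speed and amplitude.
; On overlap, CanCollide accepts only Projectile actors, printing a debug string otherwise.
; A valid hit reports the death to BP_Level2Manager and destroys the target.
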(event EventBeginPlay
  (Variables|Default|SetDirecNorm (Math|Vector|Normalize (Variables|Default|GetDirection)))
  (Variables|Default|SetOrigin (Transformation|GetActorLocation)))

(event Collision|EventActorBeginOverlap
  (params (OtherActor :type Actor%20Object%20Reference))
  (bind _cancollide (CallFunction|CanCollide OtherActor))
  (if _cancollide
    (CallFunction|OnCollide)))

(event EventTick
  (params (DeltaSeconds :type Float%20%28single-precision%29))
  (if (Variables|Default|GetIsMobile)
    (bind _output_get (Variables|Default|SetTimeCount (+ DeltaSeconds (Variables|Default|GetTimeCount))))
    (Transformation|SetActorLocation (+ (* (* (Math|Trig|Sin(Degrees) (* _output_get (Variables|Default|GetSpeed))) (Variables|Default|GetAmplitude)) (Variables|Default|GetDirecNorm)) (Variables|Default|GetOrigin)) false false)))

(event EventOnCollide
  (bind _outactors (Actor|GetAllActorsOfClass "/Game/Olaia/BP_Level2Manager.BP_Level2Manager_C"))
  (Default|AddEnemyDead _outactors)
  (Actor|DestroyActor))

(fn ConstructionScript)

(fn CanCollide
  (params (OtherActor :type Actor%20Object%20Reference))
  (Utilities|Casting|CastToProjectile OtherActor
    (:then
      (return true))
    (:CastFailed
      (Development|PrintString "Estoy cansado jefe"))))