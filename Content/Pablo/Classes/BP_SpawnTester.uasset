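; BP_SpawnTester is a simple moving actor, apparently a test object for spawning, that removes itself once it rises high enough.
; Each Tick it moves along its normalized Direction at Speed, scaled by delta time, using SetActorLocation without sweep.
; When its world Z exceeds a hard-coded threshold, it destroys itself instead of moving.
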(event EventBeginPlay)

(event Collision|EventActorBeginOverlap
  (params (OtherActor :type Actor%20Object%20Reference)))

(event EventTick
  (params (DeltaSeconds :type Float%20%28single-precision%29))
  (if (> (.z (Transformation|GetActorLocation)) 1e+02)
    (Actor|DestroyActor)
    (else
      (Transformation|SetActorLocation (+ (* (* DeltaSeconds (Variables|Default|GetSpeed)) (Math|Vector|Normalize (Variables|Default|GetDirection))) (Transformation|GetActorLocation)) false false))))

(fn ConstructionScript)