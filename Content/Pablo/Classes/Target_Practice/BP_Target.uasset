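; BP_Target is a target practice actor that destroys itself when player pawn 0 overlaps it.
; When IsMobile is set, Tick oscillates it around its starting location along the normalized Direction, using a degree-based sine of accumulated time scaled by Speed and Amplitude.
; The overlap filter and hit response are split into a CanCollide function and an OnCollide event.
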(event EventBeginPlay
  (Variables|Default|SetDirecNorm (Math|Vector|Normalize (Variables|Default|GetDirection)))
  (Variables|Default|SetOrigin (Transformation|GetActorLocation)))

(event Collision|EventActorBeginOverlap
  (params (OtherActor :type Actor%20Object%20Reference))
  (bind _cancollide (CallFunction|CanCollide OtherActor))
  (if _cancollide
    (CallFunction|OnCollide)))

(event EventTick
  (params (DeltaSeconds :type Float%20%28single-precision%29))
  (if (Variables|Default|GetIsMobile)
    (bind _output_get (Variables|Default|SetTimeCount (+ DeltaSeconds (Variables|Default|GetTimeCount))))
    (Transformation|SetActorLocation (+ (* (* (Math|Trig|Sin(Degrees) (* _output_get (Variables|Default|GetSpeed))) (Variables|Default|GetAmplitude)) (Variables|Default|GetDirecNorm)) (Variables|Default|GetOrigin)) false false)))

(event EventOnCollide
  (Actor|DestroyActor))

(fn ConstructionScript)

(fn CanCollide
  (params (OtherActor :type Actor%20Object%20Reference))
  (return (== OtherActor (Game|Player|GetPlayerPawn 0))))