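; Enemy weapon that damages the VR player on overlap while enemy-held with damage active, and that can also be grabbed in VR.
; When not enemy-held, overlap only casts to EnemyBase, with no damage applied yet.
; Grabbing enables input, adds a left- or right-hand weapon mapping context and hides that hand via a message to the controller's owner.
; Dropping reverses all three.
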(event OnGrabbed(GrabComponent)
  (bind _grabcomponent (Variables|Default|GetGrabComponent))
  (bind _returnvalue (Default|GetHeldbyHand _grabcomponent))
  (bind _returnvalue_2 (Utilities|Enum|Equal(Enum) _returnvalue "Right"))
  (Input|EnableInput (Game|GetPlayerController 0))
  (Class|BPIPawnAnim|HideUnhideHand(Message) (Components|GetOwner (Variables|/Game/VRTemplate/Blueprints/GrabComponent.GrabComponent_C|GetMotionControllerRef _grabcomponent)) true _returnvalue_2)
  (Input|AddMappingContext (PlayerController|LocalPlayerSubsystems|GetEnhancedInputLocalPlayerSubsystem (Game|GetPlayerController 0)) (select _returnvalue_2 "/Game/VRTemplate/Input/IMC_Weapon_Right.IMC_Weapon_Right" "/Game/VRTemplate/Input/IMC_Weapon_Left.IMC_Weapon_Left") 1 "(bIgnoreAllPressedKeysUntilRelease=True,bForceImmediately=False,bNotifyUserSettings=False)"))

(event OnDropped(GrabComponent)
  (bind _grabcomponent (Variables|Default|GetGrabComponent))
  (bind _returnvalue (Default|GetHeldbyHand _grabcomponent))
  (bind _returnvalue_2 (Utilities|Enum|Equal(Enum) _returnvalue "Right"))
  (Input|DisableInput (Game|GetPlayerController 0))
  (Class|BPIPawnAnim|HideUnhideHand(Message) (Components|GetOwner (Variables|/Game/VRTemplate/Blueprints/GrabComponent.GrabComponent_C|GetMotionControllerRef _grabcomponent)) false _returnvalue_2)
  (Input|RemoveMappingContext (PlayerController|LocalPlayerSubsystems|GetEnhancedInputLocalPlayerSubsystem (Game|GetPlayerController 0)) (select _returnvalue_2 "/Game/VRTemplate/Input/IMC_Weapon_Right.IMC_Weapon_Right" "/Game/VRTemplate/Input/IMC_Weapon_Left.IMC_Weapon_Left") "(bIgnoreAllPressedKeysUntilRelease=True,bForceImmediately=False,bNotifyUserSettings=False)"))

(event Collision|EventActorBeginOverlap
  (params (OtherActor :type Actor%20Object%20Reference))
  (if (Variables|Default|GetIsHeldByEnemy)
    (bind _asolaia_vrpawn (Utilities|Casting|CastToOlaiaVRPawn OtherActor))
    (if (Variables|Default|GetDamageActive)
      (Game|Damage|ApplyDamage _asolaia_vrpawn (Variables|Default|GetDamageAmount) 0 0))
    (else
      (Utilities|Casting|CastToEnemyBase OtherActor))))

(fn ConstructionScript)